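; Enemy character that chases the player and shoots arrows when its PawnSensing spots a SwapMan.
; Each sighting turns it to face the target, issues an AI move to the player and advances the cooldown for spawning an Arrow at its Sphere.
; Tick times falls to apply landing damage past a threshold, and shows a Cube while Mark is set.
; Zero health destroys it on OnTakeDMG, or flags it dead with a lifespan after fall damage.
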(event OnSeePawn(PawnSensing)
  (params (Pawn :type Pawn%20Object%20Reference))
  (bind _returnvalue (Game|Player|GetPlayerPawn 0))
  (bind _returnvalue_2 (Game|Player|GetPlayerPawn 0))
  (bind _returnvalue_3 (Transformation|GetActorRotation))
  (bind (_roll _pitch) (Math|Rotator|BreakRotator _returnvalue_3))
  (bind _asswap_man (Utilities|Casting|CastToSwapMan Pawn))
  (Transformation|SetActorRotation (Math|Rotator|MakeRotator _roll _pitch (.Yaw (Math|Rotator|BreakRotator (Math|Rotator|FindLookatRotation (Transformation|GetActorLocation) (Transformation|GetActorLocation _asswap_man))))))
  (if (<= (Variables|Default|GetAttackTimer) 0.0)
    (Game|SpawnActorfromClass "/Game/BluePrints/Arrow.Arrow_C" (Transformation|GetWorldTransform (Variables|Default|GetSphere)) "Undefined" 0 0)
    (Variables|Default|SetAttackTimer (Variables|Default|GetAttackTimerRateMax))
    (AI|AIMoveTo self (Transformation|GetActorLocation _returnvalue) _returnvalue (Variables|Default|GetRadius) false)
    (else
      (Variables|Default|SetAttackTimer (- (Variables|Default|GetAttackTimer) (* (Variables|Default|GetDT) (Variables|Default|GetAttackRate))))
      (AI|AIMoveTo self (Transformation|GetActorLocation _returnvalue_2) _returnvalue_2 (Variables|Default|GetRadius) false))))

(event Custom|OnTakeDMG
  (if (<= (Variables|Default|GetHealth) 0)
    (Actor|DestroyActor)))

(event Custom|onFallDMG
  (if (<= (Variables|Default|GetHealth) 0)
    (Variables|Default|SetDead true)
    (Actor|SetLifeSpan (Variables|Default|Getlifespanondeath))))

(event EventBeginPlay
  (Variables|/Script/Engine.CharacterMovementComponent|SetMaxWalkSpeed (Variables|Character|GetCharacterMovement) (Variables|Default|GetMovementSpeed)))

(event EventActorBeginOverlap
  (params (OtherActor :type Actor%20Object%20Reference)))

(event EventTick
  (params (DeltaSeconds :type Float%20%28single-precision%29))
  (Variables|Default|SetDT DeltaSeconds)
  (if (AI|Components|NavMovement|IsFalling (Variables|Character|GetCharacterMovement))
    (Variables|Default|SetFallTimer (+ (Variables|Default|GetFallTimer) (Variables|Default|GetDT)))
    (elif (>= (Variables|Default|GetFallTimer) (Variables|Default|GetDmgThreshhold))
      (Variables|Default|SetHealth (- (Variables|Default|GetHealth) (Math|Float|Truncate (* (- (Variables|Default|GetFallTimer) (Variables|Default|GetDmgThreshhold)) (Variables|Default|GetfallDmgMultiplier)))))
      (CallFunction|OnFallDMG)
      (Variables|Default|SetFallTimer 0.0)
      (else
        (Variables|Default|SetFallTimer 0.0))))
  (if (Variables|Default|GetMark)
    (Rendering|SetVisibility (Variables|Default|GetCube) true false)
    (else
      (Rendering|SetVisibility (Variables|Default|GetCube) false false))))

(fn ConstructionScript)